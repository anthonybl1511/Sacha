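; BP_FraiseMaster is a collectible strawberry that trails the player once collected and is banked when they are on the ground.
; Collect stores the player reference, then Tick smoothly interpolates the strawberry toward a point behind the player's capsule.
; When the player's movement reports grounded, a DoOnce calls GetStrawberry, spawns BP_StrawberryScore and destroys the actor after a short delay.
; InteractionType returns a fixed enum value.
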(event EventTick
  (params (DeltaSeconds :type Float%20%28single-precision%29))
  (bind _playerref (Variables|Default|GetplayerRef))
  (Utilities|IsValid _playerref
    (:Is%20Valid
      (Transformation|SetActorLocation (Math|Interpolation|VInterpTo (Transformation|GetActorLocation) (- (Transformation|GetActorLocation _playerref) (* (Math|Vector|GetForwardVector (Variables|/Script/Engine.Character|GetCapsuleComponent _playerref)) 1e+02)) (Utilities|Time|GetWorldDeltaSeconds) 1e+01) false false)
      (if (AI|Components|NavMovement|IsMovingonGround (Variables|/Script/Engine.Character|GetCharacterMovement (Variables|Default|GetplayerRef)))
        (Utilities|FlowControl|DoOnce false
          (:Completed
            (Default|GetStrawberry (Variables|Default|GetplayerRef))
            (Game|SpawnActorfromClass "/Game/Project/UI/BP_StrawberryScore.BP_StrawberryScore_C" (Math|Transform|MakeTransform (Transformation|GetActorLocation) "0, 0, 0" "1.000000,1.000000,1.000000") "AlwaysSpawn" "MultiplyWithRoot" 0 0)
            (Utilities|FlowControl|Delay 0.2)
            (Actor|DestroyActor)))))))

(event EventCollect
  (params (playerRef :type BP%20Player%20Object%20Reference))
  (Variables|Default|SetplayerRef playerRef))

(fn ConstructionScript)

(fn InteractionType
  (return "NewEnumerator1"))