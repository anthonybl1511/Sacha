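; BP_Fraise is a collectible strawberry that trails the player once collected and is banked when the player is on the ground.
; Collect stores the player reference, then Tick interpolates the actor toward a point behind that player's capsule.
; When the player's movement reports ground contact, a DoOnce increments the player's Fraises count and destroys the actor.
; InteractionType returns a fixed enum value identifying its interaction kind.
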(event EventTick
  (params (DeltaSeconds :type Float%20%28single-precision%29))
  (bind _playerref (Variables|Default|GetplayerRef))
  (bind _playerref_2 (Variables|Default|GetplayerRef))
  (Utilities|IsValid _playerref_2
    (:Is%20Valid
      (Transformation|SetActorLocation (Math|Interpolation|VInterpTo (Transformation|GetActorLocation) (- (Transformation|GetActorLocation _playerref_2) (* (Math|Vector|GetForwardVector (Variables|/Script/Engine.Character|GetCapsuleComponent _playerref_2)) 1e+02)) (Utilities|Time|GetWorldDeltaSeconds) 1e+01) false false)
      (if (AI|Components|NavMovement|IsMovingonGround (Variables|/Script/Engine.Character|GetCharacterMovement _playerref))
        (Utilities|FlowControl|DoOnce false
          (:Completed
            (Math|Integer|IncrementInt (Variables|/Game/Project/Character/BP_Player.BP_Player_C|Getfraises _playerref)
              (:%20%20
                (Actor|DestroyActor)))))))))

(event EventCollect
  (params (playerRef :type BP%20Player%20Object%20Reference))
  (Variables|Default|SetplayerRef playerRef))

(fn ConstructionScript)

(fn InteractionType
  (return "NewEnumerator1"))