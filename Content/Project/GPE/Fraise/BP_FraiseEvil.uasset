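; BP_FraiseEvil is an evil strawberry gameplay element that vanishes when the player dashes, extending parent behavior it calls on Tick.
; While its PlayerRef is invalid, Tick polls the player character's dashing state through a message call.
; The first detected dash triggers, via DoOnce, the Disapear timeline, which offsets the actor vertically each update and destroys it when finished.
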(event EventBeginPlay)

(event Collision|EventActorBeginOverlap
  (params (OtherActor :type Actor%20Object%20Reference)))

(event EventTick
  (params (DeltaSeconds :type Float%20%28single-precision%29))
  (|CallParentFunction DeltaSeconds)
  (Utilities|IsValid (Variables|Default|GetplayerRef)
    (:Is%20Not%20Valid
      (bind _isdashing (Class|BPIPlayer|IsDashing(Message) (Game|GetPlayerCharacter 0)))
      (if _isdashing
        (Utilities|FlowControl|DoOnce false
          (:Completed
            (bind _newtrack_0 (Timeline|disapear Play)
              (:Update
                (Transformation|AddActorWorldOffset (Math|Vector|MakeVector 0.0 0.0 (* _newtrack_0 2e+01))))
              (:Finished
                (Actor|DestroyActor)))))))))

(fn ConstructionScript
  (|CallParentFunction))