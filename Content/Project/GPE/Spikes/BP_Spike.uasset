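; BP_Spike is a hazard that sends DieMessage through BPI_Player to any overlapping actor implementing that interface.
; The construction script builds a row of collision-free static meshes with the spike material, evenly spaced along X according to SpikeLenght.
; It then positions a single Box trigger from the last child component's location and scales its extent with the length, so that box alone handles overlap detection.
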(event OnComponentBeginOverlap(Box)
  (params (OverlappedComponent :type Primitive%20Component%20Object%20Reference) (OtherActor :type Actor%20Object%20Reference) (OtherComp :type Primitive%20Component%20Object%20Reference) (OtherBodyIndex :type Integer) (bFromSweep :type Boolean) (SweepResult :type Hit%20Result%20Structure%20%28by%20ref%29))
  (if (Utilities|DoesObjectImplementInterface OtherActor "/Game/Project/Character/BPI_Player.BPI_Player_C")
    (Class|BPIPlayer|Die(Message) OtherActor)))

(event EventBeginPlay)

(event Collision|EventActorBeginOverlap
  (params (OtherActor :type Actor%20Object%20Reference)))

(event EventTick
  (params (DeltaSeconds :type Float%20%28single-precision%29)))

(fn ConstructionScript
  (bind _defaultsceneroot (Variables|Default|GetDefaultSceneRoot))
  (bind _children (Components|GetChildrenComponents _defaultsceneroot false))
  (bind _returnvalue (Utilities|Array|LastIndex _children))
  (bind _output (Utilities|Array|Get(acopy) _children _returnvalue))
  (bind _relativelocation (Variables|/Script/Engine.SceneComponent|GetRelativeLocation _output))
  (for _index (range 0 (Variables|Default|GetspikeLenght))
    (bind _returnvalue_2 (AddComponent|AddStaticMeshComponent false (Math|Transform|MakeTransform (Math|Vector|MakeVector (Math|Conversions|ToFloat(Integer) (* _index 50)) 0.0 5e+01) "0, 0, 0" "1.000000,1.000000,1.000000")))
    (Rendering|Material|SetMaterial _returnvalue_2 0 "/Game/Project/Import/Material/M_Spike.M_Spike")
    (Collision|SetCollisionEnabled _returnvalue_2 "NoCollision"))
  (Transformation|SetRelativeLocation (Variables|Default|GetBox) (Math|Vector|MakeVector (/ (.x _relativelocation) 2.0) (.y _relativelocation) (.z _relativelocation)) false false)
  (Components|Box|SetBoxExtent (Variables|Default|GetBox) (Math|Vector|MakeVector (* (+ (Math|Conversions|ToFloat(Integer) (Variables|Default|GetspikeLenght)) 1.0) 2e+01) 32.0 32.0) true))