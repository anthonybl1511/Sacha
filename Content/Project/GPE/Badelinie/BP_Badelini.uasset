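; BP_Badelini is a chaser that replays the player's path with a lag and kills the player on overlap.
; Each tick it queues the player's position; once a delay opens the gate, the sprite interpolates toward the oldest entry and removes it.
; On overlap it resets the queue and timer and moves along a spline for the lag duration before resuming the chase.
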(event OnComponentBeginOverlap(Sphere)
  (params (OverlappedComponent :type Primitive%20Component%20Object%20Reference) (OtherActor :type Actor%20Object%20Reference) (OtherComp :type Primitive%20Component%20Object%20Reference) (OtherBodyIndex :type Integer) (bFromSweep :type Boolean) (SweepResult :type Hit%20Result%20Structure%20%28by%20ref%29))
  (if (Utilities|DoesObjectImplementInterface OtherActor "/Game/Project/Character/BPI_Player.BPI_Player_C")
    (Class|BPIPlayer|Die(Message) OtherActor)
    (CallFunction|Reset)))

(event Custom|Reset
  (bind _papersprite (Variables|Default|GetPaperSprite))
  (Utilities|FlowControl|Sequence
    (:then_0
      (Variables|Default|SetmoveAlongSpline true)
      (Variables|Default|Settimer 0.0)
      (Utilities|Array|Clear (Variables|Default|GetpositionOffset))
      (Utilities|FlowControl|Gate true) ; enters at Close
    )
    (:then_1
      (Utilities|FlowControl|RetriggerableDelay (Variables|Default|GetdelayLag))
      (Variables|Default|SetmoveAlongSpline false)
      (Utilities|FlowControl|Gate true) ; enters at Open
    )))

(event EventBeginPlay
  (bind _delaylag (Variables|Default|GetdelayLag))
  (bind _papersprite (Variables|Default|GetPaperSprite))
  (Variables|/Script/Engine.SplineComponent|SetDuration (Variables|Default|GetmovementSpline) _delaylag)
  (Utilities|FlowControl|RetriggerableDelay _delaylag)
  (Variables|Default|SetmoveAlongSpline false)
  (Utilities|FlowControl|Gate true) ; enters at Open
)

(event EventTick
  (params (DeltaSeconds :type Float%20%28single-precision%29))
  (bind _papersprite (Variables|Default|GetPaperSprite))
  (Variables|Default|Settimer (+ DeltaSeconds (Variables|Default|Gettimer)))
  (if (Variables|Default|GetmoveAlongSpline)
    (Transformation|SetWorldLocation (Variables|Default|GetPaperSprite) (Spline|GetLocationatTime (Variables|Default|GetmovementSpline) (Variables|Default|Gettimer) "World" true) false false))
  (bind _location (Class|BPIPlayer|GetPlayerLoc(Message) (Game|GetPlayerCharacter 0)))
  (Utilities|Array|Add (Variables|Default|GetpositionOffset) _location)
  (Utilities|FlowControl|Gate true
    (:Exit
      (Transformation|SetWorldLocation _papersprite (Math|Interpolation|VInterpTo (Transformation|GetWorldLocation _papersprite) (Utilities|Array|Get(acopy) (Variables|Default|GetpositionOffset)) (Utilities|Time|GetWorldDeltaSeconds) 1e+01) false false)
      (Utilities|Array|RemoveIndex (Variables|Default|GetpositionOffset)))))

(fn ConstructionScript)