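; Moving platform that, when triggered, slides its cube to an offset and launches a player standing on it.
; The construction script places a preview mesh from MovingDirection on Y/Z; BeginPlay stores that location as the destination and destroys the preview.
; A speed-scaled timeline lerps the cube out, sends the launch message, then reverses after a short delay.
; A separate check waits until the cube is home to find overlapping players.
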(event Custom|resetTL
  (bind _newtrack_0 (Timeline|Timeline Reverse)
    (:Update
      (Transformation|SetRelativeLocation (Variables|Default|GetCube) (Math|Vector|Lerp(Vector) "0, 0, 0" (Variables|Default|GetfinalLocation) _newtrack_0) false false))
    (:Finished
      (if (> _newtrack_0 0.0)
        (Utilities|IsValid (Utilities|Array|Get(acopy) (Collision|GetOverlappingActors (Variables|Default|GetBox) "/Game/Project/Character/BP_Player.BP_Player_C" :!class /Script/Engine.PrimitiveComponent))
          (:Is%20Valid
            (Class|BPIPlayer|LaunchPlayer(Message) (Variables|Default|GetplayerRef) (Variables|Default|GetfinalLocation)))
          (:Is%20Not%20Valid
            (Variables|Default|SetplayerRef 0)))
        (Utilities|FlowControl|Delay 0.5)
        (CallFunction|ResetTL)))))

(event EventBeginPlay
  (bind _meshpreview (Variables|Default|GetmeshPreview))
  (|CallParentFunction)
  (Components|Timeline|SetPlayRate (Variables|Default|GetTimeline) (Variables|Default|GetplaySpeed))
  (Variables|Default|SetfinalLocation (Variables|/Script/Engine.SceneComponent|GetRelativeLocation _meshpreview))
  (Components|DestroyComponent _meshpreview))

(event EventTriggerPlateform
  (bind _newtrack_0 (Timeline|Timeline Play)
    (:Update
      (Transformation|SetRelativeLocation (Variables|Default|GetCube) (Math|Vector|Lerp(Vector) "0, 0, 0" (Variables|Default|GetfinalLocation) _newtrack_0) false false))
    (:Finished
      (if (> _newtrack_0 0.0)
        (Utilities|IsValid (Utilities|Array|Get(acopy) (Collision|GetOverlappingActors (Variables|Default|GetBox) "/Game/Project/Character/BP_Player.BP_Player_C" :!class /Script/Engine.PrimitiveComponent))
          (:Is%20Valid
            (Class|BPIPlayer|LaunchPlayer(Message) (Variables|Default|GetplayerRef) (Variables|Default|GetfinalLocation)))
          (:Is%20Not%20Valid
            (Variables|Default|SetplayerRef 0)))
        (Utilities|FlowControl|Delay 0.5)
        (CallFunction|ResetTL)))))

(fn ConstructionScript
  (bind _movingdirection (Variables|Default|GetmovingDirection))
  (|CallParentFunction)
  (Transformation|SetRelativeLocation (Variables|Default|GetmeshPreview) (Math|Vector|MakeVector 0.0 (.x _movingdirection) (.y _movingdirection)) false false))