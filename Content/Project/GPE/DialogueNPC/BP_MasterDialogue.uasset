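; BP_MasterDialogue is a dialogue NPC actor with a paper sprite that shows a subtitle message when the player interacts with it.
; A timeline started on BeginPlay animates the sprite's vertical world scale.
; Interact sends the sprite image and Dialogue text to the HUD, then after WaitingDelay tells the player to end the interaction message.
; InteractionType reports a fixed enum value.
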(event EventBeginPlay
  (bind _newtrack_0 (Timeline|Timeline Play)
    (:Update
      (Transformation|SetWorldScale3D (Variables|Default|GetPaperSprite) (Math|Vector|MakeVector 1.0 1.0 _newtrack_0)))))

(event EventInteract
  (params (playerRef :type Actor%20Object%20Reference))
  (Class|BPIHUD|ShowSubtitles(Message) (HUD|GetHUD (Game|GetPlayerController 0)) (Sprite|GetSprite (Variables|Default|GetPaperSprite)) (Variables|Default|Getdialogue))
  (Utilities|FlowControl|Delay (Variables|Default|GetwaitingDelay))
  (Class|BPIInteraction|EndInteraction(Message) playerRef))

(fn ConstructionScript)

(fn InteractionType
  (return "NewEnumerator0"))