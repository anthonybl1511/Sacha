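; BP_Player is a side-scrolling player character that moves along the Y axis with jump, wall jump and directional dash.
; BeginPlay adds the Enhanced Input mapping and copies movement, dash and camera-lag tuning from a data asset.
; Airborne after a jump, Tick box-traces both sides to set wall state for the opposing jump launch.
; Dash switches to Flying and launches along the input direction, recharging on the ground.
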(event Input|EnhancedActionEvents|EnhancedInputActionI_Move
  (params (ActionValue :type Vector%202D%20Structure) (ElapsedSeconds :type Float%20%28double-precision%29) (TriggeredSeconds :type Float%20%28double-precision%29) (InputAction :type Input%20Action%20Object%20Reference :default "/Game/Project/GameMode/Input/Input/I_Move.I_Move"))
  (Variables|Default|SetinputDirection ActionValue)
  (Pawn|Input|AddMovementInput "0.000000,1.000000,0.000000" (.X (Math|Vector2D|BreakVector2D ActionValue)) false))

(event Input|EnhancedActionEvents|EnhancedInputActionI_Jump
  (params (ActionValue :type Boolean) (ElapsedSeconds :type Float%20%28double-precision%29) (TriggeredSeconds :type Float%20%28double-precision%29) (InputAction :type Input%20Action%20Object%20Reference :default "/Game/Project/GameMode/Input/Input/I_Jump.I_Jump"))
  (:Started
    (Character|Jump)
    (if (Variables|Default|GetonWall)
      (Character|LaunchCharacter (Math|Vector|MakeVector 0.0 (Math|Conversions|ToFloat(Integer) (* (Variables|Default|GetwallDirection) -300)) (Variables|/Game/Project/Character/Metrics/DA_Player.DA_Player_C|GetjumpForce (Variables|Default|GetdataAsset))) false false)))
  (:Canceled
    (Character|StopJumping :!label _label))
  (:Completed
    (goto _label)))

(event Input|EnhancedActionEvents|EnhancedInputActionI_Dash
  (params (ActionValue :type Boolean) (ElapsedSeconds :type Float%20%28double-precision%29) (TriggeredSeconds :type Float%20%28double-precision%29) (InputAction :type Input%20Action%20Object%20Reference :default "/Game/Project/GameMode/Input/Input/I_Dash.I_Dash"))
  (bind _inputdirection (Variables|Default|GetinputDirection))
  (bind _dashforce (Variables|Default|GetdashForce))
  (:Started
    (if (Variables|Default|GetdashEnable)
      (Pawn|Components|CharacterMovement|SetMovementMode (Variables|Character|GetCharacterMovement) "MOVE_Flying" 0)
      (Character|LaunchCharacter (Math|Vector|MakeVector 0.0 (* (.x _inputdirection) _dashforce) (* (.y _inputdirection) _dashforce)) false false)
      (Variables|Default|SetdashEnable false))))

(event EventTick
  (params (DeltaSeconds :type Float%20%28single-precision%29))
  (bind _returnvalue (Transformation|GetActorLocation))
  (bind _returnvalue_2 (Transformation|GetActorLocation))
  (bind _returnvalue_3 (+ _returnvalue_2 (Math|Vector|MakeVector 0.0 1.2e+02 0.0)))
  (bind _returnvalue_4 (+ _returnvalue (Math|Vector|MakeVector 0.0 -1.2e+02 0.0)))
  (if (AI|Components|NavMovement|IsMovingonGround (Variables|Character|GetCharacterMovement))
    (Variables|Default|SetdashEnable true)
    (elif (> (Variables|Default|GetJumpCurrentCount) 0)
      (bind _returnvalue_5 (Collision|BoxTraceByChannel _returnvalue_3 _returnvalue_3 "30.000000,15.000000,75.000000" "0, 0, 0" "TraceTypeQuery1" false 0 "None"))
      (if _returnvalue_5
        (Variables|Default|SetonWall true)
        (Variables|Default|SetwallDirection 1)
        (else
          (bind _returnvalue_6 (Collision|BoxTraceByChannel _returnvalue_4 _returnvalue_4 "30.000000,15.000000,75.000000" "0, 0, 0" "TraceTypeQuery1" false 0 "None"))
          (if _returnvalue_6
            (Variables|Default|SetonWall true)
            (Variables|Default|SetwallDirection -1)
            (else
              (Variables|Default|SetonWall false))))))))

(event EventBeginPlay
  (bind _springarm (Variables|Default|GetSpringArm))
  (bind _dataasset (Variables|Default|GetdataAsset))
  (bind _charactermovement (Variables|Character|GetCharacterMovement))
  (Input|AddMappingContext (PlayerController|LocalPlayerSubsystems|GetEnhancedInputLocalPlayerSubsystem (Game|GetPlayerController 0)) "/Game/Project/GameMode/Input/IMC_Input.IMC_Input" 0 "(bIgnoreAllPressedKeysUntilRelease=True,bForceImmediately=False,bNotifyUserSettings=False)")
  (Variables|/Script/Engine.CharacterMovementComponent|SetBrakingDecelerationFlying _charactermovement (Variables|/Game/Project/Character/Metrics/DA_Player.DA_Player_C|GetbreakingFriction _dataasset))
  (Variables|/Script/Engine.CharacterMovementComponent|SetMaxWalkSpeed _charactermovement (Variables|/Game/Project/Character/Metrics/DA_Player.DA_Player_C|Getspeed _dataasset))
  (Variables|Default|SetdashForce (Variables|/Game/Project/Character/Metrics/DA_Player.DA_Player_C|Getforce _dataasset))
  (Variables|/Script/Engine.CharacterMovementComponent|SetJumpZVelocity _charactermovement (Variables|/Game/Project/Character/Metrics/DA_Player.DA_Player_C|GetjumpForce _dataasset))
  (Variables|/Script/Engine.CharacterMovementComponent|SetFallingLateralFriction _charactermovement (Variables|/Game/Project/Character/Metrics/DA_Player.DA_Player_C|GetfallingFriction _dataasset))
  (Variables|/Script/Engine.CharacterMovementComponent|SetAirControl _charactermovement (Variables|/Game/Project/Character/Metrics/DA_Player.DA_Player_C|GetairControl _dataasset))
  (Variables|/Script/Engine.CharacterMovementComponent|SetGravityScale _charactermovement (Variables|/Game/Project/Character/Metrics/DA_Player.DA_Player_C|GetgravityScale _dataasset))
  (Variables|Default|SetdashGravity (Variables|/Game/Project/Character/Metrics/DA_Player.DA_Player_C|Getgravity _dataasset))
  (Variables|/Script/Engine.SpringArmComponent|SetCameraLagSpeed _springarm (Variables|/Game/Project/Character/Metrics/DA_Player.DA_Player_C|GetcameraLag _dataasset))
  (Variables|/Script/Engine.SpringArmComponent|SetCameraLagMaxDistance _springarm (Variables|/Game/Project/Character/Metrics/DA_Player.DA_Player_C|GetcameraLagMaxDistance _dataasset)))

(fn ConstructionScript)