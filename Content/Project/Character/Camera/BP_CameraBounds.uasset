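; Camera bounds volume that hands a camera position to any overlapping actor implementing BPI_Player.
; The construction script sizes the Detection box and places the Camera from DetectionSize and CameraPosition, pulled back along X.
; BeginPlay zeroes the Camera's relative X, keeping only its Y and Z offsets.
; Begin overlap sends the Camera's world location through SetCameraPosMessage, and end overlap sends a zero vector.
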(event OnComponentBeginOverlap(detection)
  (params (OverlappedComponent :type Primitive%20Component%20Object%20Reference) (OtherActor :type Actor%20Object%20Reference) (OtherComp :type Primitive%20Component%20Object%20Reference) (OtherBodyIndex :type Integer) (bFromSweep :type Boolean) (SweepResult :type Hit%20Result%20Structure%20%28by%20ref%29))
  (if (Utilities|DoesObjectImplementInterface OtherActor "/Game/Project/Character/BPI_Player.BPI_Player_C")
    (Class|BPIPlayer|SetCameraPos(Message) OtherActor (Transformation|GetWorldLocation (Variables|Default|GetCamera)))))

(event OnComponentEndOverlap(detection)
  (params (OverlappedComponent :type Primitive%20Component%20Object%20Reference) (OtherActor :type Actor%20Object%20Reference) (OtherComp :type Primitive%20Component%20Object%20Reference) (OtherBodyIndex :type Integer))
  (if (Utilities|DoesObjectImplementInterface OtherActor "/Game/Project/Character/BPI_Player.BPI_Player_C")
    (Class|BPIPlayer|SetCameraPos(Message) OtherActor "0, 0, 0")))

(event EventBeginPlay
  (bind _camera (Variables|Default|GetCamera))
  (bind _relativelocation (Variables|/Script/Engine.SceneComponent|GetRelativeLocation _camera))
  (Transformation|SetRelativeLocation _camera (Math|Vector|MakeVector 0.0 (.y _relativelocation) (.z _relativelocation)) false false))

(fn ConstructionScript
  (bind _detectionsize (Variables|Default|GetdetectionSize))
  (bind _cameraposition (Variables|Default|GetcameraPosition))
  (Components|Box|SetBoxExtent (Variables|Default|Getdetection) (Math|Vector|MakeVector 1.2e+02 (.x _detectionsize) (.y _detectionsize)) true)
  (Transformation|SetRelativeLocation (Variables|Default|GetCamera) (Math|Vector|MakeVector (+ (.x _cameraposition) -7.5e+02) (.y _cameraposition) (.z _cameraposition)) false false))